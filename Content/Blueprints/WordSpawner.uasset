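; WordSpawner is an actor that repeatedly spawns Word actors at random heights within its Box component.
; The construction script divides the box's vertical extent into equal bands and stores a spawn point at the center of each.
; On BeginPlay, a looping timer calls Spawn Word, which spawns a Word at a randomly picked point and sets its text to a hardcoded placeholder string.
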(event EventActorBeginOverlap
  (params (OtherActor :type Actor%20Object%20Reference)))

(event EventTick
  (params (DeltaSeconds :type Float%20%28single-precision%29)))

(event EventBeginPlay
  (Utilities|Time|SetTimerbyFunctionName 0 "Spawn Word" (Variables|Default|GetSpawning%20Interval) true))

(fn ConstructionScript
  (Variables|Default|SetBoxLocation (Transformation|GetWorldLocation (Variables|Default|GetBox)))
  (Variables|Default|SetSpawn%20Point%20Offset (/ (* (.Z (Math|Vector|BreakVector (Variables|/Script/Engine.BoxComponent|GetBoxExtent (Variables|Default|GetBox)))) 2.0) (Math|Conversions|ToFloat(Integer) (Variables|Default|GetSpawn%20Point%20Amount))))
  (for _index (range 1 (Variables|Default|GetSpawn%20Point%20Amount))
    (Utilities|Array|Add (Variables|Default|GetSpawn%20Points) (Math|Vector|MakeVector (.X (Math|Vector|BreakVector (Variables|Default|GetBoxLocation))) (.Y (Math|Vector|BreakVector (Variables|Default|GetBoxLocation))) (- (+ (* _index (Variables|Default|GetSpawn%20Point%20Offset)) (- (.Z (Math|Vector|BreakVector (Variables|Default|GetBoxLocation))) (.Z (Math|Vector|BreakVector (Variables|/Script/Engine.BoxComponent|GetBoxExtent (Variables|Default|GetBox)))))) (/ (Variables|Default|GetSpawn%20Point%20Offset) 2.0))))))

(event Custom|Spawn%20Word
  (bind _spawn_points (Variables|Default|GetSpawn%20Points))
  (bind _returnvalue (Game|SpawnActorfromClass "/Game/Blueprints/Word.Word_C" (Math|Conversions|ToTransform(Vector) (Utilities|Array|Get(acopy) _spawn_points (Math|Random|RandomInteger (Utilities|Array|Length _spawn_points)))) "Undefined" 0 0))
  (Rendering|Components|TextRender|SetText (Variables|/Game/Blueprints/Word.Word_C|GetText _returnvalue) (Utilities|Text|ToText(String) "AAAA")))