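; Word killzone actor that removes words reaching its box trigger and reports them as missed.
; On begin play it caches the game state cast to NewGameState, printing an error if the cast fails.
; When an actor of exactly the Word class overlaps the box, it destroys that actor and calls WordMissed on the game state.
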(event OnComponentBeginOverlap(Box)
  (params (OtherActor :type Actor%20Object%20Reference) (OtherComp :type Primitive%20Component%20Object%20Reference) (OtherBodyIndex :type Integer) (bFromSweep :type Boolean) (SweepResult :type Hit%20Result%20Structure%20%28by%20ref%29))
  (if (== (Utilities|GetClass OtherActor) "/Game/Blueprints/Word.Word_C")
    (Actor|DestroyActor OtherActor)
    (Default|WordMissed (Variables|Default|GetGame%20State))))

(event EventBeginPlay
  (bind _asnew_game_state (Utilities|Casting|CastToNewGameState (Game|GetGameState))
    (:then
      (Variables|Default|SetGame%20State _asnew_game_state))
    (:CastFailed
      (Development|PrintText "Game State Cast Failed (WordKillZone)"))))

(event EventActorBeginOverlap
  (params (OtherActor :type Actor%20Object%20Reference)))

(event EventTick
  (params (DeltaSeconds :type Float%20%28single-precision%29)))

(fn ConstructionScript)